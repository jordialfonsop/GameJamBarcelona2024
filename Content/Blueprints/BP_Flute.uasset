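; BP_Flute is a grabbable VR flute that reports which of its colored holes the player is touching.
; While the flute is held, GetOverlappedHole checks the components overlapping the VRPawnFlute's right box, then the left box if none matched.
; It identifies green, blue, yellow or red holes by component name and returns an index, or -1 when none is found.
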(event Collision|EventActorBeginOverlap
  (params (OtherActor :type Actor%20Object%20Reference)))

(event EventTick
  (params (DeltaSeconds :type Float%20%28single-precision%29)))

(fn ConstructionScript)

(fn GetOverlappedHole
  (bind _asvrpawn_flute (Utilities|Casting|CastToVRPawnFlute (Game|Player|GetPlayerPawn 0)))
  (Variables|Default|SetHole -1)
  (if (Variables|/Game/VRTemplate/Blueprints/GrabComponent.GrabComponent_C|GetbIsHeld (Variables|Default|GetGrabComponent))
    (bind _array_element (Utilities|Array|ForEachLoopwithBreak (Class|PrimitiveComponent|GetOverlappingComponents (Variables|/Game/VRTemplate/Blueprints/VRPawnFlute.VRPawnFlute_C|GetBoxRight _asvrpawn_flute)) :!label _label)
      (:LoopBody
        (switch string (Utilities|GetObjectName _array_element)
          (:Hole%20Green
            (Variables|Default|SetHole 0)
            (goto _label Break))
          (:Hole%20Blue
            (Variables|Default|SetHole 1)
            (goto _label Break))
          (:Hole%20Yellow
            (Variables|Default|SetHole 2)
            (goto _label Break))
          (:Hole%20Red
            (Variables|Default|SetHole 3)
            (goto _label Break))))
      (:Completed
        (if (== (Variables|Default|GetHole) -1)
          (bind _array_element_2 (Utilities|Array|ForEachLoopwithBreak (Class|PrimitiveComponent|GetOverlappingComponents (Variables|/Game/VRTemplate/Blueprints/VRPawnFlute.VRPawnFlute_C|GetBoxLeft _asvrpawn_flute)) :!label _label_2)
            (:LoopBody
              (switch string (Utilities|GetObjectName _array_element_2)
                (:Hole%20Green
                  (Variables|Default|SetHole 0)
                  (goto _label_2 Break))
                (:Hole%20Blue
                  (Variables|Default|SetHole 1)
                  (goto _label_2 Break))
                (:Hole%20Yellow
                  (Variables|Default|SetHole 2)
                  (goto _label_2 Break))
                (:Hole%20Red
                  (Variables|Default|SetHole 3)
                  (goto _label_2 Break))))
            (:Completed
              _))))))
  (return (Variables|Default|GetHole)))