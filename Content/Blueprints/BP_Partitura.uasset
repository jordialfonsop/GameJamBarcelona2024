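; BP_Partitura is a musical score puzzle built from six BP_Nota child actors, each needing a matching hole and button.
; UpdatePartitura checks input against the current note, playing a cue and advancing through the first five.
; A miss or final match resets progress, refreshes all notes, plays the victory anthem and calls SetMelody; misses also play an explosion.
; SetMelody picks randomly among three cue sets, currently identical.
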(event EventBeginPlay
  (bind _asbp_nota (Utilities|Casting|CastToBP_Nota (Variables|/Script/Engine.ChildActorComponent|GetChildActor (Variables|Actor|GetBP_Nota0))))
  (Default|UpdateNote _asbp_nota)
  (bind _asbp_nota_2 (Utilities|Casting|CastToBP_Nota (Variables|/Script/Engine.ChildActorComponent|GetChildActor (Variables|Actor|GetBP_Nota1))))
  (Default|UpdateNote _asbp_nota_2)
  (bind _asbp_nota_3 (Utilities|Casting|CastToBP_Nota (Variables|/Script/Engine.ChildActorComponent|GetChildActor (Variables|Actor|GetBP_Nota2))))
  (Default|UpdateNote _asbp_nota_3)
  (bind _asbp_nota_4 (Utilities|Casting|CastToBP_Nota (Variables|/Script/Engine.ChildActorComponent|GetChildActor (Variables|Actor|GetBP_Nota3))))
  (Default|UpdateNote _asbp_nota_4)
  (bind _asbp_nota_5 (Utilities|Casting|CastToBP_Nota (Variables|/Script/Engine.ChildActorComponent|GetChildActor (Variables|Actor|GetBP_Nota4))))
  (Default|UpdateNote _asbp_nota_5)
  (bind _asbp_nota_6 (Utilities|Casting|CastToBP_Nota (Variables|/Script/Engine.ChildActorComponent|GetChildActor (Variables|Actor|GetBP_Nota5))))
  (Default|UpdateNote _asbp_nota_6)
  (CallFunction|SetMelody))

(event Collision|EventActorBeginOverlap
  (params (OtherActor :type Actor%20Object%20Reference)))

(event EventTick
  (params (DeltaSeconds :type Float%20%28single-precision%29)))

(fn ConstructionScript)

(fn UpdatePartitura
  (params (Hole :type Integer) (Button :type Integer))
  (if (!= Hole -1)
    (switch int (Variables|Default|GetCurrentStep)
      (:0
        (bind _asbp_nota (Utilities|Casting|CastToBP_Nota (Variables|/Script/Engine.ChildActorComponent|GetChildActor (Variables|Actor|GetBP_Nota0))))
        (if (== (Variables|/Game/Blueprints/BP_Nota.BP_Nota_C|GetCurrentBackground _asbp_nota) Hole)
          (if (== (Variables|/Game/Blueprints/BP_Nota.BP_Nota_C|GetCurrentNote _asbp_nota) Button)
            (Audio|PlaySound2D (Variables|Default|GetNote1) 1.0 1.0 0.0 0 0)
            (Variables|Default|SetCurrentStep (+ (Variables|Default|GetCurrentStep) 1) :!label _label)
            (else
              (Development|PrintString "FAIL" :!label _label_2)
              (Audio|PlaySound2D "/Game/StarterContent/Audio/Explosion_Cue.Explosion_Cue" 1.0 1.0 0.0 0 0)
              (Variables|Default|SetCurrentStep 0 :!label _label_3)
              (CallFunction|UpdateNotes)
              (Audio|PlaySound2D (Variables|Default|GetVictory%20Anthem) 1.0 1.0 0.0 0 0)
              (CallFunction|SetMelody)))
          (else
            (goto _label_2))))
      (:1
        (bind _asbp_nota_2 (Utilities|Casting|CastToBP_Nota (Variables|/Script/Engine.ChildActorComponent|GetChildActor (Variables|Actor|GetBP_Nota1))))
        (if (== (Variables|/Game/Blueprints/BP_Nota.BP_Nota_C|GetCurrentBackground _asbp_nota_2) Hole)
          (if (== (Variables|/Game/Blueprints/BP_Nota.BP_Nota_C|GetCurrentNote _asbp_nota_2) Button)
            (Audio|PlaySound2D (Variables|Default|GetNote2) 1.0 1.0 0.0 0 0)
            (goto _label)
            (else
              (goto _label_2)))
          (else
            (goto _label_2))))
      (:2
        (bind _asbp_nota_3 (Utilities|Casting|CastToBP_Nota (Variables|/Script/Engine.ChildActorComponent|GetChildActor (Variables|Actor|GetBP_Nota2))))
        (if (== (Variables|/Game/Blueprints/BP_Nota.BP_Nota_C|GetCurrentBackground _asbp_nota_3) Hole)
          (if (== (Variables|/Game/Blueprints/BP_Nota.BP_Nota_C|GetCurrentNote _asbp_nota_3) Button)
            (Audio|PlaySound2D (Variables|Default|GetNote3) 1.0 1.0 0.0 0 0)
            (goto _label)
            (else
              (goto _label_2)))
          (else
            (goto _label_2))))
      (:3
        (bind _asbp_nota_4 (Utilities|Casting|CastToBP_Nota (Variables|/Script/Engine.ChildActorComponent|GetChildActor (Variables|Actor|GetBP_Nota3))))
        (if (== (Variables|/Game/Blueprints/BP_Nota.BP_Nota_C|GetCurrentBackground _asbp_nota_4) Hole)
          (if (== (Variables|/Game/Blueprints/BP_Nota.BP_Nota_C|GetCurrentNote _asbp_nota_4) Button)
            (Audio|PlaySound2D (Variables|Default|GetNote4) 1.0 1.0 0.0 0 0)
            (goto _label)
            (else
              (goto _label_2)))
          (else
            (goto _label_2))))
      (:4
        (bind _asbp_nota_5 (Utilities|Casting|CastToBP_Nota (Variables|/Script/Engine.ChildActorComponent|GetChildActor (Variables|Actor|GetBP_Nota4))))
        (if (== (Variables|/Game/Blueprints/BP_Nota.BP_Nota_C|GetCurrentBackground _asbp_nota_5) Hole)
          (if (== (Variables|/Game/Blueprints/BP_Nota.BP_Nota_C|GetCurrentNote _asbp_nota_5) Button)
            (Audio|PlaySound2D (Variables|Default|GetNote5) 1.0 1.0 0.0 0 0)
            (goto _label)
            (else
              (goto _label_2)))
          (else
            (goto _label_2))))
      (:5
        (bind _asbp_nota_6 (Utilities|Casting|CastToBP_Nota (Variables|/Script/Engine.ChildActorComponent|GetChildActor (Variables|Actor|GetBP_Nota5))))
        (if (== (Variables|/Game/Blueprints/BP_Nota.BP_Nota_C|GetCurrentBackground _asbp_nota_6) Hole)
          (if (== (Variables|/Game/Blueprints/BP_Nota.BP_Nota_C|GetCurrentNote _asbp_nota_6) Button)
            (Development|PrintString "SUCCESS")
            (goto _label_3)
            (else
              (goto _label_2)))
          (else
            (goto _label_2)))))))

(fn UpdateNotes
  (bind _asbp_nota (Utilities|Casting|CastToBP_Nota (Variables|/Script/Engine.ChildActorComponent|GetChildActor (Variables|Actor|GetBP_Nota0))))
  (Default|UpdateNote _asbp_nota)
  (bind _asbp_nota_2 (Utilities|Casting|CastToBP_Nota (Variables|/Script/Engine.ChildActorComponent|GetChildActor (Variables|Actor|GetBP_Nota1))))
  (Default|UpdateNote _asbp_nota_2)
  (bind _asbp_nota_3 (Utilities|Casting|CastToBP_Nota (Variables|/Script/Engine.ChildActorComponent|GetChildActor (Variables|Actor|GetBP_Nota2))))
  (Default|UpdateNote _asbp_nota_3)
  (bind _asbp_nota_4 (Utilities|Casting|CastToBP_Nota (Variables|/Script/Engine.ChildActorComponent|GetChildActor (Variables|Actor|GetBP_Nota3))))
  (Default|UpdateNote _asbp_nota_4)
  (bind _asbp_nota_5 (Utilities|Casting|CastToBP_Nota (Variables|/Script/Engine.ChildActorComponent|GetChildActor (Variables|Actor|GetBP_Nota4))))
  (Default|UpdateNote _asbp_nota_5)
  (bind _asbp_nota_6 (Utilities|Casting|CastToBP_Nota (Variables|/Script/Engine.ChildActorComponent|GetChildActor (Variables|Actor|GetBP_Nota5))))
  (Default|UpdateNote _asbp_nota_6))

(fn SetMelody
  (switch int (Math|Random|RandomIntegerinRange 0 2)
    (:0
      (CallFunction|SetSoundCues "/Game/Audio/Melodias/Melodia_1/SC_Victory.SC_Victory" "/Game/Audio/Melodias/Melodia_1/SC_1.SC_1" "/Game/Audio/Melodias/Melodia_1/SC_2.SC_2" "/Game/Audio/Melodias/Melodia_1/SC_3.SC_3" "/Game/Audio/Melodias/Melodia_1/SC_4.SC_4" "/Game/Audio/Melodias/Melodia_1/SC_5.SC_5"))
    (:1
      (CallFunction|SetSoundCues "/Game/Audio/Melodias/Melodia_2/SC_Victory.SC_Victory" "/Game/Audio/Melodias/Melodia_2/SC_1.SC_1" "/Game/Audio/Melodias/Melodia_2/SC_2.SC_2" "/Game/Audio/Melodias/Melodia_2/SC_3.SC_3" "/Game/Audio/Melodias/Melodia_2/SC_4.SC_4" "/Game/Audio/Melodias/Melodia_2/SC_5.SC_5"))
    (:2
      (CallFunction|SetSoundCues "/Game/Audio/Melodias/Melodia_3/SC_Victory.SC_Victory" "/Game/Audio/Melodias/Melodia_3/SC_1.SC_1" "/Game/Audio/Melodias/Melodia_3/SC_2.SC_2" "/Game/Audio/Melodias/Melodia_3/SC_3.SC_3" "/Game/Audio/Melodias/Melodia_3/SC_4.SC_4" "/Game/Audio/Melodias/Melodia_3/SC_5.SC_5"))))

(fn SetSoundCues
  (params (Melody :type Sound%20Cue%20Object%20Reference) (Note1 :type Sound%20Cue%20Object%20Reference) (Note2 :type Sound%20Cue%20Object%20Reference) (Note3 :type Sound%20Cue%20Object%20Reference) (Note4 :type Sound%20Cue%20Object%20Reference) (Note5 :type Sound%20Cue%20Object%20Reference))
  (Variables|Default|SetVictory%20Anthem Melody)
  (Variables|Default|SetNote1 Note1)
  (Variables|Default|SetNote2 Note2)
  (Variables|Default|SetNote3 Note3)
  (Variables|Default|SetNote4 Note4)
  (Variables|Default|SetNote5 Note5))