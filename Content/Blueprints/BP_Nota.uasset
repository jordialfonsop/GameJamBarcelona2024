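; Note actor that displays a randomly chosen button symbol over a randomly chosen colored background.
; UpdateNote rolls random indices within the ButtonTypes and ColorTypes arrays, storing them as CurrentNote and CurrentBackground.
; SetNoteAndBackgroundParams hides every component, then reveals the matching one of three notes and four backgrounds.
; The event graph and construction script are empty, so nothing in this Blueprint calls UpdateNote.
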(event EventBeginPlay)

(event Collision|EventActorBeginOverlap
  (params (OtherActor :type Actor%20Object%20Reference)))

(event EventTick
  (params (DeltaSeconds :type Float%20%28single-precision%29)))

(fn ConstructionScript)

(fn GetRandomValues
  (bind _output_get (Variables|Default|SetCurrentBackground (Math|Random|RandomIntegerinRange 0 (- (Utilities|Set|Length (Variables|Default|GetColor%20Types)) 1))))
  (bind _output_get_2 (Variables|Default|SetCurrentNote (Math|Random|RandomIntegerinRange 0 (- (Utilities|Set|Length (Variables|Default|GetButton%20Types)) 1))))
  (return _output_get _output_get_2))

(fn SetAllInvisible
  (Rendering|SetVisibility (Variables|Default|GetBackground3) false false)
  (Rendering|SetVisibility (Variables|Default|GetBackground2) false false)
  (Rendering|SetVisibility (Variables|Default|GetBackground1) false false)
  (Rendering|SetVisibility (Variables|Default|GetBackground0) false false)
  (Rendering|SetVisibility (Variables|Default|GetNote2) false false)
  (Rendering|SetVisibility (Variables|Default|GetNote1) false false)
  (Rendering|SetVisibility (Variables|Default|GetNote0) false false))

(fn SetNoteandBackgroundParams
  (params (Button :type Integer) (Color :type Integer))
  (CallFunction|SetAllInvisible)
  (switch int Button
    (:0
      (Rendering|SetVisibility (Variables|Default|GetNote0) true false))
    (:1
      (Rendering|SetVisibility (Variables|Default|GetNote1) true false))
    (:2
      (Rendering|SetVisibility (Variables|Default|GetNote2) true false)))
  (switch int Color
    (:0
      (Rendering|SetVisibility (Variables|Default|GetBackground0) true false))
    (:1
      (Rendering|SetVisibility (Variables|Default|GetBackground1) true false))
    (:2
      (Rendering|SetVisibility (Variables|Default|GetBackground2) true false))
    (:3
      (Rendering|SetVisibility (Variables|Default|GetBackground3) true false))))

(fn UpdateNote
  (bind (_color _button) (CallFunction|GetRandomValues))
  (CallFunction|SetAllInvisible)
  (CallFunction|SetNoteandBackgroundParams _button _color))